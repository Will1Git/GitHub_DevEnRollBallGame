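; Base pawn for a physics-driven ball that the player rolls relative to the camera's direction.
; Move axis inputs apply mass-independent force to the static mesh along the camera's forward and right vectors, scaled by MoveSpeed.
; Turn and look axes feed controller yaw and pitch.
; Inactive world-axis movement events and disconnected impulse nodes remain as reference samples.
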(event `InputAxis|Move_ForwardBack`
  (params (AxisValue :type "Float (single-precision)"))
  ;[0 0 0] Move Forward Back - V02 - Moves with Camera - Ball will now only move relative to the Camera Direction! Feels like the Camera Follows the Ball
  ;;[1 1 1] Add force works well with Input Actions because. Add force shuld be called every frame and the Input Event do that. For managable Force to have effect either Chaneg the Mass of the Mesh to much less that 1 or Taggle the Ignore mass (Accel Change) Attribute in the node.
  (`PrimitiveComponent.AddForce` (`self.StaticMesh`) (* (* (`SceneComponent.GetForwardVector` (`self.Camera`)) AxisValue) (`self.MoveSpeed`)) "None" true))

(event `CustomEvent`
  (params (`Axis Value` :type "Float (single-precision)"))
  ;[0 0 0] Move Forward Back - V01 - Non-Active Sample
  ; Simple Version - WORKS BUT Does not move with Player/Camera
  ; This Only moves in Absolute World Y Direction - So When you turn around you conrolls are bacward etc...
  ;;[1 1 1] Add force works well with Input Actions because. Add force shuld be called every frame and the Input Event do that. For managable Force to have effect either Chaneg the Mass of the Mesh to much less that 1 or Toggle the Ignore mass (Accel Change) Attribute in the node.
  (`PrimitiveComponent.AddForce` (`self.StaticMesh`) (* (`KismetMathLibrary.MakeVector` `Axis Value`) (`self.MoveSpeed`)) "None" true))

(event `CustomEvent_1`
  (params (`Axis Value` :type "Float (single-precision)"))
  ;[0 0 0] Move Right Left - V01 - Non-Active Sample
  ;;[1 1 1] Add force works well with Input Actions because. Add force shuld be called every frame and the Input Event do that. For managable Force to have effect either Chaneg the Mass of the Mesh to much less that 1 or Toggle the Ignore mass (Accel Change) Attribute in the node.
  (`PrimitiveComponent.AddForce` (`self.StaticMesh`) (* (`KismetMathLibrary.MakeVector` 0.0 `Axis Value`) (`self.MoveSpeed`)) "None" true))

(event `InputAxis|Move_RightLeft`
  (params (AxisValue :type "Float (single-precision)"))
  ;[0 0 0] Move Right Left - V02 - Moves with Camera - Ball will now only move relative to the Camera Direction! Feels like the Camera Follows the Ball
  ;;[1 1 1] Add force works well with Input Actions because. Add force shuld be called every frame and the Input Event do that. For managable Force to have effect either Chaneg the Mass of the Mesh to much less that 1 or Toggle the Ignore mass (Accel Change) Attribute in the node.
  (`PrimitiveComponent.AddForce` (`self.StaticMesh`) (* (* (`SceneComponent.GetRightVector` (`self.Camera`)) AxisValue) (`self.MoveSpeed`)) "None" true))

(event `InputAxis|Turn_RightLeft`
  (params (AxisValue :type "Float (single-precision)"))
  ;[0 0 0] Turn Right Left - V01
  (`self.AddControllerYawInput` AxisValue))

(event `InputAxis|Look_UpDown`
  (params (AxisValue :type "Float (single-precision)"))
  ;[0 0 0] Look Up Down - V01
  (`self.AddControllerPitchInput` AxisValue))

(fn `UserConstructionScript`)
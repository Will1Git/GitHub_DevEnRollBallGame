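; BP_EventTickTest_Movement is a test actor that demonstrates frame-rate independent movement along world X.
; Tick drives the active version, adding a world offset of MoveSpeed scaled by DeltaSeconds.
; Two earlier SetActorLocation versions remain for comparison: an unconnected per-frame one without delta time, and a delta-scaled one on FakeEventTick, which nothing in this graph calls.
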(event `FakeEventTick`
  (params (DeltaSeconds :type "Float (single-precision)"))
  ;[1 1 1] V02 - This Sample Shows Deltal Time Multipled - Using PROPER TIME in Seconds
  (`self.K2_SetActorLocation` (+ (`self.K2_GetActorLocation`) (`KismetMathLibrary.MakeVector` (* DeltaSeconds (`self.MoveSpeed`))))))

(event `self.ReceiveTick`
  (params (DeltaSeconds :type "Float (single-precision)"))
  ;[1 1 1] V03 - Using the Simplified Add Actor World Offset - Meaning we can skip the Additions part and the Get Actor Location Part as the node does that Already.
  ; BUT IMPORTANT: We Still need to Mutilply the Delta Time From Tick (Even if thr Node Says Delta Times!!!)
  (`self.K2_AddActorWorldOffset` (`KismetMathLibrary.MakeVector` (* DeltaSeconds (`self.MoveSpeed`)))))

(fn `UserConstructionScript`)